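; Master enemy character that chases the player and attacks with either a spawned projectile or direct damage, gated by a cooldown.
; Tick issues AIMoveTo every frame and attacks within range; an alternative TickAI event exists, but its looping timer is never run.
; Damage feeds the health component, whose death event grants the player health and shield, then destroys the enemy.
; An elite flag doubles health and enlarges the capsule.
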(event `Attack_Player`
  (bind _returnvalue (`self.K2_GetActorLocation`))
  ;[0.15 0.15 0.15 0.5 98] Enemy  System
  ;;[0.638 0.01128 0 0.5 62] Enemy Damage System
  ;;; Enemies damaging to the player
  (if (`self.CanAttack?`)
    (set `self.CanAttack?` false)
    (if (`self.IsRanged`)
      (bind _asbp_character (cast `/Game/Dynamic/Character/Character_Blueprints/BP_Character` (`GameplayStatics.GetPlayerCharacter` 0)))
      (bind _returnvalue_2 (`|SpawnActorFromClass` "/Game/Dynamic/Ai/AI_Unique/Projectiles/BP_EnemyProjectile.BP_EnemyProjectile_C" (`KismetMathLibrary.MakeTransform` _returnvalue (`KismetMathLibrary.FindLookAtRotation` _returnvalue (`self.K2_GetActorLocation` _asbp_character))) "Undefined" "MultiplyWithRoot" self null))
      (set `/Game/Dynamic/Ai/AI_Unique/Projectiles/BP_EnemyProjectile.Shooter_REF` self _returnvalue_2)
      (`KismetSystemLibrary.Delay` (`self.AttackCooldown`))
      (set `self.CanAttack?` true)
      (else
        (bind _asbp_character_2 (cast `/Game/Dynamic/Character/Character_Blueprints/BP_Character` (`GameplayStatics.GetPlayerCharacter` 0)))
        (`GameplayStatics.ApplyDamage` _asbp_character_2 (`self.AttackDamage`))
        (`KismetSystemLibrary.Delay` (`self.AttackCooldown`))
        (set `self.CanAttack?` true)))))

(event `self.AC_HealthSystem.OnDeath`
  ;[0.15 0.15 0.15 0.5 98] Enemy  System
  ;; Enemy Death if reaches 0 and Enemy as a resource
  (bind _asbp_character (cast `/Game/Dynamic/Character/Character_Blueprints/BP_Character` (`GameplayStatics.GetPlayerCharacter` 0)))
  (`/Game/Dynamic/Character/Character_Blueprints/BP_Character.GainHealthAndShield` _asbp_character 15.0)
  (`self.K2_DestroyActor`))

(event `self.ReceiveBeginPlay`
  (bind _ac_healthsystem (`self.AC_HealthSystem`))
  (bind _returnvalue (* (`self.MaxHealth`) 2.0))
  ;[0.15 0.15 0.15 0.5 98] Enemy  System
  (`self.SpawnDefaultController`)
  (`KismetSystemLibrary.PrintString` (`KismetStringLibrary.Conv_BoolToString` (`KismetSystemLibrary.IsValid` (`self.GetController`))))
  (bind _asbp_character (cast `/Game/Dynamic/Character/Character_Blueprints/BP_Character` (`GameplayStatics.GetPlayerCharacter` 0)))
  (set `self.PlayerREF` _asbp_character)
  ;; Enemy Health
  (if (`self.IsElite?`)
    (set `/Game/Dynamic/Character/Character_Blueprints/AC_HealthSystem.CurrentHealth` _returnvalue _ac_healthsystem)
    (set `/Game/Dynamic/Character/Character_Blueprints/AC_HealthSystem.MaxHealth` _returnvalue _ac_healthsystem)
    (else
      (set `/Game/Dynamic/Character/Character_Blueprints/AC_HealthSystem.CurrentHealth` (`self.MaxHealth`) (`self.AC_HealthSystem`))))
  (set `CharacterMovementComponent.MaxWalkSpeed` (`self.MovementSpeed`) (`self.CharacterMovement`)))

(event `self.ReceiveAnyDamage`
  (params (Damage :type "Float (single-precision)") (DamageType :type "DamageType Object Reference") (InstigatedBy :type "Controller Object Reference") (DamageCauser :type "Actor Object Reference"))
  ;[0.15 0.15 0.15 0.5 98] Enemy  System
  ;;[0.638 0.01128 0 0.5 62] Enemy Damage System
  ;;; Enemies getting damage
  (`KismetSystemLibrary.PrintString` (`KismetStringLibrary.Concat_StrStr` (`KismetSystemLibrary.GetDisplayName` self) ".   " (`KismetStringLibrary.Conv_DoubleToString` Damage)))
  (message `/Game/Dynamic/Character/Input/Interfaces/BPI_Damage.TakeDamage_Interfaces` (`self.AC_HealthSystem`) Damage null))

(event `Tick AI`
  ;[0.15 0.15 0.15 0.5 98] Enemy  System
  (`/Engine/EditorBlueprintResources/StandardMacros.IsValid` (`self.PlayerREF`)
    (:`Is Valid`
      (if (<= (`KismetMathLibrary.VSize` (- (`self.K2_GetActorLocation`) (`self.K2_GetActorLocation` (`self.PlayerREF`)))) (`self.AttackRange`))
        (`Controller.StopMovement` (`self.GetController`))
        (`self.Attack_Player`)
        (`KismetSystemLibrary.PrintString` "Attacking")
        (else
          (bind _movementresult (`|AIMoveTo` self (0.0 0.0 0.0) (`self.PlayerREF`) (`self.AttackRange`) true)
            (:`OnSuccess`
              (`KismetSystemLibrary.PrintString` "MoveTo Success"))
            (:`OnFail`
              (`KismetSystemLibrary.PrintString` (`|GetEnumeratorNameAsString` _movementresult)))))))))

(event `self.ReceiveTick`
  (params (DeltaSeconds :type "Float (single-precision)"))
  (bind _returnvalue (`GameplayStatics.GetPlayerCharacter` 0))
  (bind _attackrange (`self.AttackRange`))
  (bind _returnvalue_2 (`self.K2_GetActorLocation` _returnvalue))
  ; Move and Attack
  (`/Engine/EditorBlueprintResources/StandardMacros.IsValid` _returnvalue
    (:`Is Valid`
      (bind _movementresult (`|AIMoveTo` self _returnvalue_2 _returnvalue _attackrange)
        (:`then`
          (if (<= (`KismetMathLibrary.VSize` (- _returnvalue_2 (`self.K2_GetActorLocation`))) _attackrange)
            (`self.Attack_Player`)))
        (:`OnSuccess`
          (`KismetSystemLibrary.PrintString` "Move To Success"))))))

(fn `UserConstructionScript`
  (if (`self.IsElite?`)
    (`SceneComponent.SetWorldScale3D` (`self.CapsuleComponent`) (1.5 1.5 1.5))
    (else
      (`SceneComponent.SetWorldScale3D` (`self.CapsuleComponent`) (1.0 1.0 1.0)))))