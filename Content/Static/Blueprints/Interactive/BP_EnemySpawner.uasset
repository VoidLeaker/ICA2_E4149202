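; Enemy spawner actor that, when active at BeginPlay, periodically spawns an enemy class until a count limit or duration is reached.
; A looping timer calls SpawnEnemy, while a second timer calls StopSpawner to deactivate it.
; Both random offset axes use SpawnRadius as min and max, so spawns land at one fixed diagonal offset.
; Stopping clears SpawnTimerHandle, though BeginPlay never assigns that handle.
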(event `self.ReceiveBeginPlay`
  (if (`self.bSpawnActive`)
    (`KismetSystemLibrary.K2_SetTimer` null "SpawnEnemy" (`self.SpawnInterval`) true)
    (`KismetSystemLibrary.K2_SetTimer` null "StopSpawner" (`self.SpawnerDuration`))))

(fn `SpawnEnemy`
  (if (`self.bSpawnActive`)
    (if (>= (`self.SpawnCount`) (`self.MaxSpawnCount`))
      (set `self.bSpawnActive` false)
      (`KismetSystemLibrary.K2_ClearAndInvalidateTimerHandle` (`self.SpawnTimerHandle`))
      (return)
      (else
        (`|SpawnActorFromClass` (`self.EnemyClass`) (`KismetMathLibrary.MakeTransform` (+ (`self.K2_GetActorLocation`) (`KismetMathLibrary.MakeVector` (`KismetMathLibrary.RandomFloatInRange` (`self.SpawnRadius`) (`self.SpawnRadius`)) (`KismetMathLibrary.RandomFloatInRange` (`self.SpawnRadius`) (`self.SpawnRadius`)))) (`self.K2_GetActorRotation`)) "Undefined" "MultiplyWithRoot" null null)
        (set `self.SpawnCount` (+ (`self.SpawnCount`) 1))))
    (else
      (`KismetSystemLibrary.K2_ClearAndInvalidateTimerHandle` (`self.SpawnTimerHandle`))
      (return))))

(fn `StopSpawner`
  (set `self.bSpawnActive` false)
  (`KismetSystemLibrary.K2_ClearAndInvalidateTimerHandle` (`self.SpawnTimerHandle`)))

(fn `UserConstructionScript`)