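; Explosive barrel actor that takes damage and explodes when its health runs out.
; AnyDamage subtracts from BarrelCurrentHealth and calls Explode at zero or below.
; Explode applies radial damage at the barrel's location, draws a debug sphere for the radius, then destroys the actor.
; Debug prints trace each step; the IsDestroyed flag is set but its check is left unwired.
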(event `self.ReceiveAnyDamage`
  (params (Damage :type "Float (single-precision)") (DamageType :type "DamageType Object Reference") (InstigatedBy :type "Controller Object Reference") (DamageCauser :type "Actor Object Reference"))
  (`KismetSystemLibrary.PrintString` "Barrel called")
  (bind _output_get (set `self.BarrelCurrentHealth` (- (`self.BarrelCurrentHealth`) Damage)))
  (`KismetSystemLibrary.PrintString` (`KismetStringLibrary.Conv_DoubleToString` _output_get) true true (struct :`G` 0.66 :`B` 1.0 :`A` 1.0) _output_get)
  (if (<= _output_get 0.0)
    (`KismetSystemLibrary.PrintString` "BOOM!")
    (`self.Explode`)
    (else
      (`KismetSystemLibrary.PrintString` "Not Working"))))

(event `Explode`
  (bind _returnvalue (`self.K2_GetActorLocation`))
  (bind _damageradius (`self.DamageRadius`))
  (set `self.bIsDestroyed?` true)
  (`GameplayStatics.ApplyRadialDamage` :`BaseDamage` (`self.ExplosionDamage`) :`Origin` _returnvalue :`DamageRadius` _damageradius :`DamageTypeClass` "/Script/Engine.DamageType" :`DamageCauser` null :`InstigatedByController` null)
  (`KismetSystemLibrary.DrawDebugSphere` _returnvalue _damageradius 12 (struct :`R` 1.0 :`G` 1.0 :`B` 1.0 :`A` 1.0) 1.0)
  (`self.K2_DestroyActor`)
  (`KismetSystemLibrary.PrintString` "Barrel Destroy"))

(fn `UserConstructionScript`)