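; BP_BFGProjectile is the BFG weapon's projectile, which deals area damage when it touches something other than its shooter.
; On sphere overlap, provided the Shooter is valid, it applies radial damage at its location using its Damage, Radius and DamageType, ignoring the Shooter, then destroys itself.
; The BP_Enemy_Master cast does not affect the result, and a debug sphere draw is left disconnected.
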(event `self.SphereCollision.OnComponentBeginOverlap`
  (params (OverlappedComponent :type "PrimitiveComponent Object Reference") (OtherActor :type "Actor Object Reference") (OtherComp :type "PrimitiveComponent Object Reference") (OtherBodyIndex :type Integer) (bFromSweep :type Boolean) (SweepResult :type "HitResult Structure (by ref)"))
  (bind _shooter (`self.Shooter`))
  (if (`KismetSystemLibrary.IsValid` _shooter)
    (if (!= OtherActor _shooter)
      (cast `/Game/Dynamic/Ai/Common_Enemies/BP_Enemy_Master` OtherActor
        (:`then`
          _)
        (:`CastFailed`
          _))
      (`GameplayStatics.ApplyRadialDamage` (`self.Damage`) (`self.K2_GetActorLocation`) (`self.Radius`) "/Script/Engine.DamageType" (`|MakeArray` _shooter :!type "Actor Object Reference") self null)
      (`self.K2_DestroyActor`))))

(event `self.ReceiveBeginPlay`)

(fn `UserConstructionScript`)